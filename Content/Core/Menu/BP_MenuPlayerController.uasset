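; Player controller for the main menu that creates and shows the menu widget for the local player.
; On BeginPlay it adds WBP_Menu to the viewport, switches to UI-only input and shows the mouse cursor.
; If the EOS lobby subsystem reports the player is already in a lobby, it switches the menu's main switcher to its second page.
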(event `self.ReceiveBeginPlay`
  (if (`self.IsLocalPlayerController`)
    (bind _returnvalue (`|CreateWidget` "/Game/UI/WBP_Menu.WBP_Menu_C" self))
    (`UserWidget.AddToViewport` _returnvalue 0)
    (`WidgetBlueprintLibrary.SetInputMode_UIOnlyEx` self null)
    (set `self.bShowMouseCursor` true)
    (if (`EOSLobbySubsystem.IsInLobby` (subsystem `EOSLobbySubsystem`))
      (`WidgetSwitcher.SetActiveWidgetIndex` (`/Game/UI/WBP_Menu.MainSwitcher` _returnvalue) 1))))

(fn `CreateAndShowHUD`
  (returns (MenuRef :type "/Game/UI/WBP_Menu Object Reference"))
  (return null))

(fn `UserConstructionScript`)
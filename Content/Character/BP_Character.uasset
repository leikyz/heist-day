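; Networked player character with sprinting, health, a toggleable rifle with aiming, and carryable keycards and props.
; Server events validate interactions through BPI_Interactable with a facing check, and detach held items to drop or throw them, briefly disabling prop pawn collision and impact damage on throws.
; Lethal damage drops held items and ragdolls the body via multicast and OnRep.
; Rifle fire only runs a debug-drawn camera trace, without applying damage.
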(event Custom|Server_TryInteract
  (params (TargetActor :type Actor%20Object%20Reference))
  (bind _self self)
  ;[0.15 0.15 0.15 0.5] Réponse interaction pour serveur multi
  (if (not (Variables|Default|GetIsDead))
    (Utilities|IsValid TargetActor
      (:Is%20Valid
        (if (Utilities|DoesObjectImplementInterface TargetActor "/Game/Gameplay/Interaction/BPI_Interactable.BPI_Interactable_C")
          (if (>= (Math|Vector|DotProduct (Math|Vector|Normalize (- (Transformation|GetActorLocation TargetActor) (Transformation|GetActorLocation))) (Math|Vector|GetForwardVector (Pawn|GetControlRotation (Pawn|GetController) :!class /Script/Engine.Controller))) 0.3)
            (bind _return_value (Class|BPIInteractable|CanInteract(Message) TargetActor _self))
            (if _return_value
              (Class|BPIInteractable|Interact(Message) TargetActor _self))))))))

(event Custom|Server_DropKeycard
  ;[0.15 0.15 0.15 0.5] Drop la keycard au sol devant soit et pouvoir la reprendre (reset les utilisations etc)
  (Development|PrintString "SERVER DROP")
  (Utilities|IsValid (Variables|Default|GetHeldKeycard)
    (:Is%20Valid
      (Transformation|DetachFromActor (Variables|Default|GetHeldKeycard) "KeepWorld" "KeepWorld" "KeepWorld")
      (Rendering|SetActorHiddenInGame (Variables|Default|GetHeldKeycard) false)
      (Collision|SetActorEnableCollision (Variables|Default|GetHeldKeycard) true)
      (Physics|SetSimulatePhysics (Variables|/Game/Gameplay/Items/Keycard/BP_KeycardPickup.BP_KeycardPickup_C|GetCube (Variables|Default|GetHeldKeycard)) true)
      (Transformation|SetActorTransform (Variables|Default|GetHeldKeycard) (Math|Transform|MakeTransform (+ (Transformation|GetActorLocation) (* (Transformation|GetActorForwardVector) (Variables|Default|Getfloat%20120)) (Math|Vector|MakeVector -5e+01 0.0 3e+01)) (Transformation|GetActorRotation) "0.250000,0.250000,0.250000") false true)
      (Networking|ForceNetUpdate (Variables|Default|GetHeldKeycard))
      (Networking|FlushNetDormancy (Variables|Default|GetHeldKeycard))
      (Variables|Default|SetHeldKeycard 0))))

(event Custom|StartAim
  ;[0.15 0.15 0.15 0.5] Aim
  (switch Utilities|FlowControl|Switch|SwitchonE_Weapon_Type (Variables|Default|GetE_WeaponType)
    (:NewEnumerator1
      (Variables|Default|SetbIsAiming true)
      (Variables|/Script/Engine.CharacterMovementComponent|SetMaxWalkSpeed (Variables|Character|GetCharacterMovement) (Variables|Default|GetAimWalkSpeed))
      (Variables|Default|SetbIsSprinting false))))

(event Custom|ToggleWeapon
  ;[0.15 0.15 0.15 0.5] Weapon Cycling
  (switch Utilities|FlowControl|Switch|SwitchonE_Weapon_Type (Variables|Default|GetE_WeaponType)
    (:NewEnumerator0
      (Rendering|SetVisibility (Variables|Default|GetSKM_Rifle) true false)
      (Variables|Default|SetE_WeaponType "NewEnumerator1"))
    (:NewEnumerator1
      (Rendering|SetVisibility (Variables|Default|GetSKM_Rifle) false false)
      (Variables|Default|SetE_WeaponType "NewEnumerator0"))))

(event Custom|Server_ReceiveDamage
  (params (DamageAmount :type Float%20%28double-precision%29))
  ;[0.15 0.15 0.15 0.5] Recevoir des degats d'objet coté reseaux/client
  (CallFunction|ReceiveDamage DamageAmount))

(event Custom|Server_ThrowProp
  ;[0.15 0.15 0.15 0.5] Lancer un item loin devant soi (paramètrer les props directement via leur BP)
  (Utilities|IsValid (Variables|Default|GetHeldProp)
    (:Is%20Valid
      (Class|Actor|SetReplicateMovement (Variables|Default|GetHeldProp) true)
      (Networking|ForceNetUpdate (Variables|Default|GetHeldProp))
      (Networking|FlushNetDormancy (Variables|Default|GetHeldProp))
      (Default|MulticastDetachfromHolder (Variables|Default|GetHeldProp))
      (Collision|SetCollisionResponsetoChannel (Variables|/Game/Gameplay/Items/Props/BP_CarryableBase.BP_CarryableBase_C|GetPropMesh (Variables|Default|GetHeldProp)) "ECC_Pawn" "ECR_Ignore")
      (Variables|/Game/Gameplay/Items/Props/BP_CarryableBase.BP_CarryableBase_C|SetCanDealImpactNow (Variables|Default|GetHeldProp) false)
      (Physics|AddImpulse (Variables|/Game/Gameplay/Items/Props/BP_CarryableBase.BP_CarryableBase_C|GetPropMesh (Variables|Default|GetHeldProp)) (+ (* (Transformation|GetActorUpVector) (Variables|Default|GetVector%20Force)) (* (Transformation|GetActorForwardVector) (Variables|/Game/Gameplay/Items/Props/BP_CarryableBase.BP_CarryableBase_C|GetThrowForce (Variables|Default|GetHeldProp)))) "None" true)
      (Utilities|Time|SetTimerbyFunctionName (Variables|Default|GetHeldProp) "EnableImpactDamage" 0.2)
      (Utilities|Time|SetTimerbyFunctionName (Variables|Default|GetHeldProp) "RestorePawnCollision" 0.2)
      (Variables|Default|SetHeldProp 0))))

(event Custom|Server_DropProp
  ;[0.15 0.15 0.15 0.5] Drop un item au sol et pouvoir le reprendre (comme la keycard)
  (Utilities|IsValid (Variables|Default|GetHeldProp)
    (:Is%20Valid
      (Class|Actor|SetReplicateMovement (Variables|Default|GetHeldProp) true)
      (Networking|ForceNetUpdate (Variables|Default|GetHeldProp))
      (Networking|FlushNetDormancy (Variables|Default|GetHeldProp))
      (Default|MulticastDetachfromHolder (Variables|Default|GetHeldProp))
      (Variables|Default|SetHeldProp 0))))

(event Custom|FireWeapon
  (bind _camera (Variables|Default|GetCamera))
  (bind _returnvalue (Transformation|GetWorldLocation _camera))
  ;[0.15 0.15 0.15 0.5] Weapon Firing
  (switch Utilities|FlowControl|Switch|SwitchonE_Weapon_Type (Variables|Default|GetE_WeaponType)
    (:NewEnumerator1
      (Collision|MultiLineTraceByChannel _returnvalue (+ _returnvalue (* (Math|Vector|GetForwardVector (Pawn|GetControlRotation (Pawn|GetController) :!class /Script/Engine.Controller)) "1000.000000,1000.000000,1000.000000")) "TraceTypeQuery1" false 0 "ForDuration"))))

(event Custom|StartSprint
  ;[0.15 0.15 0.15 0.5] Sprint
  (if (not (Variables|Default|GetbIsAiming))
    (Variables|Default|SetbIsSprinting true)
    (Variables|/Script/Engine.CharacterMovementComponent|SetMaxWalkSpeed (Variables|Character|GetCharacterMovement) (Variables|Default|GetSprintSpeed))))

(event Custom|StopSprint
  ;[0.15 0.15 0.15 0.5] Sprint
  (if (not (Variables|Default|GetbIsAiming))
    (Variables|Default|SetbIsSprinting false)
    (Variables|/Script/Engine.CharacterMovementComponent|SetMaxWalkSpeed (Variables|Character|GetCharacterMovement) (Variables|Default|GetWalkSpeed))))

(event Custom|Multicast_EnterRagdoll
  ;[0.15 0.15 0.15 0.5] Ragdoll coté serveur
  (CallFunction|EnterRagdoll))

(event Custom|StopAim
  ;[0.15 0.15 0.15 0.5] Aim
  (switch Utilities|FlowControl|Switch|SwitchonE_Weapon_Type (Variables|Default|GetE_WeaponType)
    (:NewEnumerator1
      (Variables|Default|SetbIsAiming false)
      (Variables|/Script/Engine.CharacterMovementComponent|SetMaxWalkSpeed (Variables|Character|GetCharacterMovement) (Variables|Default|GetWalkSpeed)))))

(event EventBeginPlay
  ;[0.15 0.15 0.15 0.5] Defaults
  (Variables|/Script/Engine.CharacterMovementComponent|SetMaxWalkSpeed (Variables|Character|GetCharacterMovement) (Variables|Default|GetWalkSpeed))
  (Variables|Default|SetCurrentHealth (Variables|Default|GetMaxHealth))
  (Rendering|SetVisibility (Variables|Default|GetSKM_Rifle) false false)
  ;[0.15 0.15 0.15 0.5] Debug (leik add)
  (Development|ExecuteConsoleCommand "stat fps" (Game|GetPlayerController 0)))

(event Collision|EventActorBeginOverlap
  (params (OtherActor :type Actor%20Object%20Reference)))

(event EventTick
  (params (DeltaSeconds :type Float%20%28single-precision%29)))

(event Input|KeyboardEvents|DebugKeyF1
  (params (Key :type Key%20Structure :default "None") (ActionValue :type Input%20Action%20Value%20Structure))
  ;[0.15 0.15 0.15 0.5] Debug (leik add)
  (:Pressed
    (Development|ExecuteConsoleCommand "EnableCheats" (Game|GetPlayerController 0))
    (Development|ExecuteConsoleCommand "r.ShadowQuality 0" (Game|GetPlayerController 0))))

(fn ConstructionScript)

(fn ReceiveDamage
  (params (DamageAmount :type Float%20%28double-precision%29))
  ;[0.15 0.15 0.15 0.5] Si plus de vie apres degats recu = mort
  (if (not (Variables|Default|GetIsDead))
    (bind _output_get (Variables|Default|SetCurrentHealth (- (Variables|Default|GetCurrentHealth) DamageAmount)))
    (Development|PrintString (Utilities|String|ToString(Float) _output_get))
    (if (<= (Variables|Default|GetCurrentHealth) 0.0)
      (Utilities|FlowControl|Sequence
        (:then_0
          (Utilities|IsValid (Variables|Default|GetHeldProp)
            (:Is%20Valid
              (CallFunction|ServerDropProp))
            (:Is%20Not%20Valid
              _)))
        (:then_1
          (Utilities|IsValid (Variables|Default|GetHeldKeycard)
            (:Is%20Valid
              (CallFunction|ServerDropKeycard))
            (:Is%20Not%20Valid
              _))))
      (Variables|Default|SetIsDead true)
      (CallFunction|MulticastEnterRagdoll))))

(fn EnterRagdoll
  (Pawn|Components|CharacterMovement|DisableMovement (Variables|Character|GetCharacterMovement))
  (Collision|SetCollisionEnabled (Variables|Collision|GetCapsuleComponent) "NoCollision")
  (Collision|SetCollisionProfileName (Variables|Character|GetMesh) "Ragdoll" true :!class /Script/Engine.PrimitiveComponent)
  (Physics|SetSimulatePhysics (Variables|Character|GetMesh) true))

(fn OnRepIsDead
  ;[0.15 0.15 0.15 0.5] Mettre ragdoll multi ready
  (if (Variables|Default|GetIsDead)
    (CallFunction|EnterRagdoll)))
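; Player controller for BP_Character that maps Enhanced Input to movement, look, sprint, weapon, prop and keycard actions, plus spectator view cycling.
; It creates the local team-score HUD and shows popups and timer-refreshed action hints and keycard uses on it.
; A looping camera line trace outlines BPI_Interactable targets and shows prompts.
; Interact uses a sphere trace, then calls the character's server event, as do drop and aimed throw.
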(event `self.ReceiveBeginPlay`
  ; Defaults/Binds
  (if (`self.IsLocalPlayerController`)
    (`WidgetBlueprintLibrary.SetInputMode_GameOnly` self)
    (set `self.bShowMouseCursor` false)
    (`EnhancedInputSubsystemInterface.AddMappingContext` (pcsubsystem `EnhancedInputLocalPlayerSubsystem` self) "/Game/Character/Control/Input/IMC_Player.IMC_Player" 0 (struct))
    (bind _returnvalue (`|CreateWidget` "/Game/UI/WBP_TeamScore.WBP_TeamScore_C" self))
    (bind _output_get (set `self.HUDWidgetRef` _returnvalue))
    (`UserWidget.AddToViewport` _output_get 0)
    (`self.UpdateActionHints`)
    (`KismetSystemLibrary.K2_SetTimer` null "UpdateInteractionPrompt" 0.1 true)
    (`KismetSystemLibrary.K2_SetTimer` null "UpdateActionHints" 0.1 true)))

(event `EnhancedInput|/Game/Character/Control/Input/IA_SwitchSpectatorMode`
  (params (ActionValue :type Boolean) (ElapsedSeconds :type "Float (double-precision)") (TriggeredSeconds :type "Float (double-precision)") (InputAction :type "InputAction Object Reference" :default "/Game/Character/Control/Input/IA_SwitchSpectatorMode.IA_SwitchSpectatorMode"))
  ;[0.15 0.09735 0.03663 0.5] SwitchjSpectatorMode
  (:`Triggered`
    (bind _outactors (`GameplayStatics.GetAllActorsOfClass` "/Game/Character/BP_Character.BP_Character_C"))
    (bind _result (`/Engine/EditorBlueprintResources/StandardMacros.IncrementInt` (`self.Target Index`))
      (:`  `
        (if (> _result (`KismetArrayLibrary.Array_LastIndex` _outactors))
          (set `self.Target Index` 0))
        (`self.SetViewTargetWithBlend` (`|GetArrayItem` _outactors (`self.Target Index`)))))))

(event `UpdateInteractionPrompt`
  (bind _currentoutlinedinteractable (`self.CurrentOutlinedInteractable`))
  ; Promp UI + Outline prop ect
  (bind _asbp_character (cast `/Game/Character/BP_Character` (`self.K2_GetPawn`))
    (:`then`
      (if (`/Game/Character/BP_Character.IsDead` _asbp_character)
        (`self.ClearInteractionState`)
        (else
          (bind _returnvalue (`SceneComponent.K2_GetComponentLocation` (`/Game/Character/BP_Character.Camera` _asbp_character)))
          (bind _outhit (`KismetSystemLibrary.LineTraceSingle` _returnvalue (+ _returnvalue (* (`KismetMathLibrary.GetForwardVector` (`SceneComponent.K2_GetComponentRotation` (`/Game/Character/BP_Character.Camera` _asbp_character))) (`/Game/Character/BP_Character.InteractTraceDistance` _asbp_character))) "TraceTypeQuery2" false (`|MakeArray` _asbp_character :!type "Actor Object Reference")))
          (bind (_bblockinghit _binitialoverlap _time _distance _location _impactpoint _normal _impactnormal _physmat _hitactor) (`GameplayStatics.BreakHitResult` _outhit))
          (`/Engine/EditorBlueprintResources/StandardMacros.IsValid` _hitactor
            (:`Is Valid`
              (if (`KismetSystemLibrary.DoesImplementInterface` _hitactor "/Game/Gameplay/Interaction/BPI_Interactable.BPI_Interactable_C")
                (bind _return_value (message `/Game/Gameplay/Interaction/BPI_Interactable.CanInteract` _hitactor _asbp_character))
                (if _return_value
                  (if (!= _currentoutlinedinteractable _hitactor)
                    (`/Engine/EditorBlueprintResources/StandardMacros.IsValid` _currentoutlinedinteractable
                      (:`Is Valid`
                        (message `/Game/Gameplay/Interaction/BPI_Interactable.SetOutlineEnable` _currentoutlinedinteractable false)
                        (message `/Game/Gameplay/Interaction/BPI_Interactable.SetOutlineEnable` _hitactor true)
                        (set `self.CurrentOutlinedInteractable` _hitactor)
                        (bind _interactiontext (message `/Game/Gameplay/Interaction/BPI_Interactable.GetInteractionText` _hitactor _asbp_character))
                        (`/Game/UI/WBP_TeamScore.ShowInteractionPrompt` (`self.HUDWidgetRef`) _interactiontext))
                      (:`Is Not Valid`
                        (message `/Game/Gameplay/Interaction/BPI_Interactable.SetOutlineEnable` _hitactor true)
                        (set `self.CurrentOutlinedInteractable` _hitactor)
                        (bind _interactiontext_2 (message `/Game/Gameplay/Interaction/BPI_Interactable.GetInteractionText` _hitactor _asbp_character))
                        (`/Game/UI/WBP_TeamScore.ShowInteractionPrompt` (`self.HUDWidgetRef`) _interactiontext_2)))
                    (else
                      (bind _interactiontext_3 (message `/Game/Gameplay/Interaction/BPI_Interactable.GetInteractionText` _hitactor _asbp_character))
                      (`/Game/UI/WBP_TeamScore.ShowInteractionPrompt` (`self.HUDWidgetRef`) _interactiontext_3)))
                  (else
                    (`self.ClearInteractionState`)))
                (else
                  (`self.ClearInteractionState`))))
            (:`Is Not Valid`
              (`self.ClearInteractionState`))))))
    (:`CastFailed`
      (`self.ClearInteractionState`))))

(event `EnhancedInput|/Game/Character/Control/Input/IA_Interaction`
  (params (ActionValue :type Boolean) (ElapsedSeconds :type "Float (double-precision)") (TriggeredSeconds :type "Float (double-precision)") (InputAction :type "InputAction Object Reference" :default "/Game/Character/Control/Input/IA_Interaction.IA_Interaction"))
  ; Tracer la ligne pour interagir avec un objet interactable
  (:`Started`
    (bind _asbp_character (cast `/Game/Character/BP_Character` (`self.K2_GetPawn`)))
    (bind _returnvalue (`SceneComponent.K2_GetComponentLocation` (`/Game/Character/BP_Character.Camera` _asbp_character)))
    (bind _outhit (`KismetSystemLibrary.SphereTraceSingle` _returnvalue (+ _returnvalue (* (`KismetMathLibrary.GetForwardVector` (`SceneComponent.K2_GetComponentRotation` (`/Game/Character/BP_Character.Camera` _asbp_character))) (`/Game/Character/BP_Character.InteractTraceDistance` _asbp_character))) (`/Game/Character/BP_Character.InteractTraceRadius` _asbp_character) "TraceTypeQuery2" false (`|MakeArray` _asbp_character :!type "Actor Object Reference") "ForDuration"))
    (bind (_bblockinghit _binitialoverlap _time _distance _location _impactpoint _normal _impactnormal _physmat _hitactor) (`GameplayStatics.BreakHitResult` _outhit))
    (`/Engine/EditorBlueprintResources/StandardMacros.IsValid` _hitactor
      (:`Is Valid`
        (if (`KismetSystemLibrary.DoesImplementInterface` _hitactor "/Game/Gameplay/Interaction/BPI_Interactable.BPI_Interactable_C")
          (bind _asbp_character_2 (cast `/Game/Character/BP_Character` (`self.K2_GetPawn`)))
          (`/Game/Character/BP_Character.Server_TryInteract` _asbp_character_2 _hitactor))))))

(event `Client_ShowActionPopup`
  (params (Message :type Text))
  (bind _hudwidgetref (`self.HUDWidgetRef`))
  ; Afficher popup keycard client
  (`/Engine/EditorBlueprintResources/StandardMacros.IsValid` _hudwidgetref
    (:`Is Valid`
      (`/Game/UI/WBP_TeamScore.ShowKeycardPopup` _hudwidgetref Message))))

(event `EnhancedInput|/Game/Character/Control/Input/IA_Move`
  (params (ActionValue :type "Vector2D Structure") (ElapsedSeconds :type "Float (double-precision)") (TriggeredSeconds :type "Float (double-precision)") (InputAction :type "InputAction Object Reference" :default "/Game/Character/Control/Input/IA_Move.IA_Move"))
  (bind (_x _y) (`KismetMathLibrary.BreakVector2D` ActionValue))
  (bind _returnvalue (`self.K2_GetPawn`))
  (bind _returnvalue_2 (`KismetMathLibrary.MakeRotator` 0.0 0.0 (.yaw (`self.GetControlRotation`))))
  ; Movement
  (:`Triggered`
    (`Pawn.AddMovementInput` _returnvalue (`KismetMathLibrary.GetForwardVector` _returnvalue_2) _y false)
    (`Pawn.AddMovementInput` _returnvalue (`KismetMathLibrary.GetRightVector` _returnvalue_2) _x false)))

(event `EnhancedInput|/Game/Character/Control/Input/IA_DropKeycard`
  (params (ActionValue :type Boolean) (ElapsedSeconds :type "Float (double-precision)") (TriggeredSeconds :type "Float (double-precision)") (InputAction :type "InputAction Object Reference" :default "/Game/Character/Control/Input/IA_DropKeycard.IA_DropKeycard"))
  ; Input pour drop la keycard au sol
  (:`Started`
    (bind _asbp_character (cast `/Game/Character/BP_Character` (`self.K2_GetPawn`)))
    (`/Game/Character/BP_Character.Server_DropKeycard` _asbp_character)))

(event `ShowExtractionPopupLocal`
  (params (Amount :type Integer))
  (bind _hudwidgetref (`self.HUDWidgetRef`))
  ; Afficher $ extraction local
  (`/Engine/EditorBlueprintResources/StandardMacros.IsValid` _hudwidgetref
    (:`Is Valid`
      (`/Game/UI/WBP_TeamScore.ShowExtractionPopup` _hudwidgetref Amount))))

(event `EnhancedInput|/Game/Character/Control/Input/IA_DropProp`
  (params (ActionValue :type Boolean) (ElapsedSeconds :type "Float (double-precision)") (TriggeredSeconds :type "Float (double-precision)") (InputAction :type "InputAction Object Reference" :default "/Game/Character/Control/Input/IA_DropProp.IA_DropProp"))
  ; Input pour drop un prop
  (:`Started`
    (bind _asbp_character (cast `/Game/Character/BP_Character` (`self.K2_GetPawn`)))
    (`/Game/Character/BP_Character.Server_DropProp` _asbp_character)))

(event `EnhancedInput|/Game/Character/Control/Input/IA_Look`
  (params (ActionValue :type "Vector2D Structure") (ElapsedSeconds :type "Float (double-precision)") (TriggeredSeconds :type "Float (double-precision)") (InputAction :type "InputAction Object Reference" :default "/Game/Character/Control/Input/IA_Look.IA_Look"))
  (bind (_x _y) (`KismetMathLibrary.BreakVector2D` ActionValue))
  (bind _returnvalue (`self.K2_GetPawn`))
  ; Camera
  (:`Triggered`
    (bind _result (`/Engine/EditorBlueprintResources/StandardMacros.NegateFloat` _y)
      (:`  `
        (`/Engine/EditorBlueprintResources/StandardMacros.IsValid` _returnvalue
          (:`Is Valid`
            (`Pawn.AddControllerYawInput` _returnvalue _x)
            (`Pawn.AddControllerPitchInput` _returnvalue _result)))))))

(event `EnhancedInput|/Game/Character/Control/Input/IA_Throw`
  (params (ActionValue :type Boolean) (ElapsedSeconds :type "Float (double-precision)") (TriggeredSeconds :type "Float (double-precision)") (InputAction :type "InputAction Object Reference" :default "/Game/Character/Control/Input/IA_Throw.IA_Throw"))
  ; Input pour lancer un prop la ou on vise avec camera
  (:`Started`
    (bind _asbp_character (cast `/Game/Character/BP_Character` (`self.K2_GetPawn`)))
    (bind _camera (`/Game/Character/BP_Character.Camera` _asbp_character))
    (bind _returnvalue (`SceneComponent.K2_GetComponentLocation` _camera))
    (bind _returnvalue_2 (+ _returnvalue (* (`SceneComponent.GetForwardVector` _camera) (`self.AimTraceDistance`))))
    (bind (_outhit _returnvalue_3) (`KismetSystemLibrary.LineTraceSingle` :`Start` _returnvalue :`End` _returnvalue_2 :`TraceChannel` "TraceTypeQuery1" :`DrawDebugType` "ForDuration"))
    (`/Game/Character/BP_Character.Server_ThrowProp` _asbp_character (`KismetMathLibrary.SelectVector` _returnvalue_2 (`.ImpactPoint` (`GameplayStatics.BreakHitResult` _outhit)) _returnvalue_3))))

(event `EnhancedInput|/Game/Character/Control/Input/IA_CycleWeapon`
  (params (ActionValue :type Boolean) (ElapsedSeconds :type "Float (double-precision)") (TriggeredSeconds :type "Float (double-precision)") (InputAction :type "InputAction Object Reference" :default "/Game/Character/Control/Input/IA_CycleWeapon.IA_CycleWeapon"))
  ; Weapon Cycling
  (:`Started`
    (bind _asbp_character (cast `/Game/Character/BP_Character` (`self.K2_GetPawn`)))
    (`/Game/Character/BP_Character.ToggleWeapon` _asbp_character)))

(event `EnhancedInput|/Game/Character/Control/Input/IA_Sprint`
  (params (ActionValue :type Boolean) (ElapsedSeconds :type "Float (double-precision)") (TriggeredSeconds :type "Float (double-precision)") (InputAction :type "InputAction Object Reference" :default "/Game/Character/Control/Input/IA_Sprint.IA_Sprint"))
  ; Sprint
  (:`Started`
    (bind _asbp_character (cast `/Game/Character/BP_Character` (`self.K2_GetPawn`)))
    (`/Game/Character/BP_Character.StartSprint` _asbp_character))
  (:`Canceled`
    (`/Game/Character/BP_Character.StopSprint` _asbp_character :!label _label))
  (:`Completed`
    (goto _label)))

(event `EnhancedInput|/Game/Character/Control/Input/IA_Aim`
  (params (ActionValue :type Boolean) (ElapsedSeconds :type "Float (double-precision)") (TriggeredSeconds :type "Float (double-precision)") (InputAction :type "InputAction Object Reference" :default "/Game/Character/Control/Input/IA_Aim.IA_Aim"))
  ; Aim
  (:`Started`
    (bind _asbp_character (cast `/Game/Character/BP_Character` (`self.K2_GetPawn`)))
    (`/Game/Character/BP_Character.StartAim` _asbp_character))
  (:`Canceled`
    (`/Game/Character/BP_Character.StopAim` _asbp_character :!label _label_2))
  (:`Completed`
    (goto _label_2)))

(event `EnhancedInput|/Game/Character/Control/Input/IA_Fire`
  (params (ActionValue :type Boolean) (ElapsedSeconds :type "Float (double-precision)") (TriggeredSeconds :type "Float (double-precision)") (InputAction :type "InputAction Object Reference" :default "/Game/Character/Control/Input/IA_Fire.IA_Fire"))
  ; Weapon Firing
  (:`Triggered`
    (bind _asbp_character (cast `/Game/Character/BP_Character` (`self.K2_GetPawn`)))
    (`/Game/Character/BP_Character.FireWeapon` _asbp_character)))

(fn `ClearInteractionState`
  (bind _currentoutlinedinteractable (`self.CurrentOutlinedInteractable`))
  (`/Engine/EditorBlueprintResources/StandardMacros.IsValid` _currentoutlinedinteractable
    (:`Is Valid`
      (message `/Game/Gameplay/Interaction/BPI_Interactable.SetOutlineEnable` _currentoutlinedinteractable false)
      (set `self.CurrentOutlinedInteractable` null)
      (`/Game/UI/WBP_TeamScore.HideInteractionPopup` (`self.HUDWidgetRef`)))
    (:`Is Not Valid`
      (set `self.CurrentOutlinedInteractable` null)
      (`/Game/UI/WBP_TeamScore.HideInteractionPopup` (`self.HUDWidgetRef`)))))

(fn `UpdateActionHints`
  (bind _hudwidgetref (`self.HUDWidgetRef`))
  ; Afficher touche d'interaction prop/keycard
  (bind _asbp_character (cast `/Game/Character/BP_Character` (`self.K2_GetPawn`)))
  (if (`KismetSystemLibrary.IsValid` (`/Game/Character/BP_Character.HeldProp` _asbp_character))
    (if (`/Game/Character/BP_Character.IsInExtractionZone` _asbp_character)
      (bind _heldkeycard (`/Game/Character/BP_Character.HeldKeycard` _asbp_character))
      (bind _returnvalue (`KismetSystemLibrary.IsValid` _heldkeycard))
      (`/Game/UI/WBP_TeamScore.UpdateActionHints` (`self.HUDWidgetRef`) true true _returnvalue "Extract")
      (else
        (`/Game/UI/WBP_TeamScore.UpdateActionHints` (`self.HUDWidgetRef`) true true _returnvalue "Drop")))
    (else
      (`/Game/UI/WBP_TeamScore.UpdateActionHints` (`self.HUDWidgetRef`) false false _returnvalue "")))
  (if _returnvalue
    (switch `/Game/Gameplay/E_Player_Team` (`/Game/Character/BP_Character.Team` _asbp_character)
      (:`NewEnumerator0`
        (`/Game/UI/WBP_TeamScore.UpdateKeycardUses` _hudwidgetref true (`|FormatText` "x{Value}" (`KismetTextLibrary.Conv_IntToText` (`/Game/Gameplay/Items/Keycard/BP_KeycardPickup.UsesRemaining_Attackers` _heldkeycard)))))
      (:`NewEnumerator1`
        (`/Game/UI/WBP_TeamScore.UpdateKeycardUses` _hudwidgetref false "")))
    (else
      (`/Game/UI/WBP_TeamScore.UpdateKeycardUses` _hudwidgetref false ""))))

(fn `UserConstructionScript`)
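; Extraction zone actor where thieves deposit carryable props to score for their team.
; Box overlaps toggle each BP_Character's IsInExtractionZone flag.
; TryExtractProp runs on authority, requires an extractable, released prop whose last holder is a Thief, then has the GameMode award the team score and handle the robbery.
; An older GameState-based scoring chain remains in the EventGraph but is disconnected.
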(event `self.Box.OnComponentBeginOverlap`
  (params (OverlappedComponent :type "PrimitiveComponent Object Reference") (OtherActor :type "Actor Object Reference") (OtherComp :type "PrimitiveComponent Object Reference") (OtherBodyIndex :type Integer) (bFromSweep :type Boolean) (SweepResult :type "HitResult Structure (by ref)"))
  ; Système d'extraction que si overlap entre prop et zone donc pas opti
  (bind _asbp_character (cast `/Game/Character/BP_Character` OtherActor))
  (set `/Game/Character/BP_Character.IsInExtractionZone` true _asbp_character))

(event `self.Box.OnComponentEndOverlap`
  (params (OverlappedComponent :type "PrimitiveComponent Object Reference") (OtherActor :type "Actor Object Reference") (OtherComp :type "PrimitiveComponent Object Reference") (OtherBodyIndex :type Integer))
  ; Sortir de la zone = plus d'affichage extract
  (bind _asbp_character (cast `/Game/Character/BP_Character` OtherActor))
  (set `/Game/Character/BP_Character.IsInExtractionZone` false _asbp_character))

(fn `TryExtractProp`
  (params (Props :type "/Game/Gameplay/Items/Props/BP_CarryableBase Object Reference"))
  (returns (WasExtracted :type Boolean))
  (bind _lastholder (`/Game/Gameplay/Items/Props/BP_CarryableBase.LastHolder` Props))
  ; Condition d'extraction d'objet pour donner les points
  (`/Engine/EditorBlueprintResources/ActorMacros.Switch Has Authority`
    (:`Authority`
      (if (`/Game/Gameplay/Items/Props/BP_CarryableBase.CanBeExtracted` Props)
        (if (`/Game/Gameplay/Items/Props/BP_CarryableBase.IsHeld` Props)
          (return false)
          (else
            (bind _asheist_day_game_state (cast `HeistDayGameState` (`GameplayStatics.GetGameState`)))
            (bind _asheist_day_player_state (cast `HeistDayPlayerState` (`Pawn.PlayerState` _lastholder)))
            (cast `/Game/BP_GameState` _asheist_day_game_state)
            (bind _asheist_day_game_mode (cast `HeistDayGameMode` (`GameplayStatics.GetGameMode`)))
            (if (`|EnumEquality` (`HeistDayPlayerState.GetTeam` _asheist_day_player_state) "Thief")
              (`HeistDayGameMode.AwardThiefScore` _asheist_day_game_mode (`HeistDayPlayerState.GetTeamId` _asheist_day_player_state) (`/Game/Gameplay/Items/Props/BP_CarryableBase.ExtractionValue` Props))
              (`HeistDayGameMode.HandlePlayerRobbed` _asheist_day_game_mode (`Pawn.GetController` _lastholder))
              (return true)
              (else
                (return false)))))
        (else
          (return false))))))

(fn `UserConstructionScript`)
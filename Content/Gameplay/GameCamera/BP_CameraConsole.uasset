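; BP_CameraConsole is an interactable security camera console that lets players on the Employee team cycle through a list of cameras.
; On remote clients, BeginPlay creates the camera widget, registers the console with the player controller and enables render-texture writing only on the first camera.
; Interact, swap and leave check the team, call OnInteract or NavigateCamera, and show, relabel or remove the widget.
; Leaving also re-enables render-texture writing on the current camera.
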(event `self.ReceiveBeginPlay`
  (bind _cameralist (`self.CameraList`))
  (`/Engine/EditorBlueprintResources/ActorMacros.Switch Has Authority`
    (:`Remote`
      (`KismetSystemLibrary.PrintString` "affichage bp")
      (bind _returnvalue (`|CreateWidget` "/Game/UI/WBP_Camera.WBP_Camera_C" (`GameplayStatics.GetPlayerController` 0)))
      (bind _output_get (set `self.Widget` _returnvalue))
      (`/Game/UI/WBP_Camera.SetCameraTxt` _output_get (`self.IndexCamera`))
      (bind _asbp_character_controller (cast `/Game/Character/Control/BP_CharacterController` (`GameplayStatics.GetPlayerController` 0)))
      (set `/Game/Character/Control/BP_CharacterController.BP_CameraConsole` self _asbp_character_controller)
      (for _array_element _cameralist
        (bind _asbp_camera (cast `/Game/Gameplay/GameCamera/BP_Camera` _array_element))
        (`/Game/Gameplay/GameCamera/BP_Camera.WriteRenderTexture` _asbp_camera false))
      (bind _asbp_camera_2 (cast `/Game/Gameplay/GameCamera/BP_Camera` (`|GetArrayItem` _cameralist)))
      (`/Game/Gameplay/GameCamera/BP_Camera.WriteRenderTexture` _asbp_camera_2 true))))

(fn `CameraInteract`
  (returns (CameraPawn :type "Pawn Object Reference"))
  (bind _returnvalue (`GameplayStatics.GetPlayerPawn` 0))
  (bind _asbp_character (cast `/Game/Character/BP_Character` _returnvalue))
  (switch `ETeam` (`HeistDayPlayerState.GetTeam` (`/Game/Character/BP_Character.As Heist Day Player State` _asbp_character))
    (:`Employee`
      (bind _returnvalue_2 (`self.OnInteract` true _returnvalue))
      (`UserWidget.AddToViewport` (`self.Widget`) 0)
      (return _returnvalue_2))))

(fn `GetInteractionText`
  (params (Interactor :type "Actor Object Reference"))
  (returns (InteractionText :type Text))
  (return ""))

(fn `LeaveCamera`
  (returns (PlayerPawn :type "Pawn Object Reference"))
  (bind _asbp_character (cast `/Game/Character/BP_Character` (`self.PlayerPawn`)))
  (switch `ETeam` (`HeistDayPlayerState.GetTeam` (`/Game/Character/BP_Character.As Heist Day Player State` _asbp_character))
    (:`Employee`
      (bind _returnvalue (`self.OnInteract` false))
      (bind _asbp_camera (cast `/Game/Gameplay/GameCamera/BP_Camera` (`|GetArrayItem` (`self.CameraList`) (`self.IndexCamera`))))
      (`/Game/Gameplay/GameCamera/BP_Camera.WriteRenderTexture` _asbp_camera true)
      (`Widget.RemoveFromParent` (`self.Widget`))
      (return _returnvalue))))

(fn `ShouldPlayInteractionSound`
  (returns (Bool :type Boolean))
  (return false))

(fn `SwapCamera`
  (params (StepDir :type Integer))
  (returns (CameraPawn :type "Pawn Object Reference"))
  (bind _asbp_character (cast `/Game/Character/BP_Character` (`self.PlayerPawn`)))
  (switch `ETeam` (`HeistDayPlayerState.GetTeam` (`/Game/Character/BP_Character.As Heist Day Player State` _asbp_character))
    (:`Employee`
      (bind _returnvalue (`self.NavigateCamera` StepDir))
      (`/Engine/EditorBlueprintResources/StandardMacros.IsValid` _returnvalue
        (:`Is Valid`
          (`/Game/UI/WBP_Camera.SetCameraTxt` (`self.Widget`) (`self.IndexCamera`))
          (return _returnvalue))))))

(fn `UserConstructionScript`)
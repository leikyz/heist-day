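; BP_Camera is a possessable, rotatable in-game camera that feeds a scene capture into the RT_Camera render texture.
; It assigns that texture as the capture target only while possessed, clearing it on unpossess.
; On BeginPlay it offsets its yaw and pitch limits by the starting rotation.
; IA_Look input adds to the current rotation and passes through ClampCameraAngle with those limits before setting actor rotation.
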(event `self.ReceiveUnpossessed`
  (params (OldController :type "Controller Object Reference"))
  (`self.WriteRenderTexture` false))

(event `self.ReceivePossessed`
  (params (NewController :type "Controller Object Reference"))
  (`self.WriteRenderTexture` true))

(event `self.ReceiveBeginPlay`
  (bind (_returnvalue_roll _returnvalue_pitch _returnvalue_yaw) (`KismetMathLibrary.BreakRotator` (`self.K2_GetActorRotation`)))
  (bind _returnvalue (`KismetMathLibrary.MakeVector2D` _returnvalue_yaw _returnvalue_pitch))
  (set `self.RotationMin` (+ _returnvalue (`self.RotationMin`)))
  (set `self.RotationMax` (+ _returnvalue (`self.RotationMax`))))

(event `EnhancedInput|/Game/Character/Control/Input/IA_Look`
  (params (ActionValue :type "Vector2D Structure") (ElapsedSeconds :type "Float (double-precision)") (TriggeredSeconds :type "Float (double-precision)") (InputAction :type "InputAction Object Reference" :default "/Game/Character/Control/Input/IA_Look.IA_Look"))
  (bind (_returnvalue_roll _returnvalue_pitch _returnvalue_yaw) (`KismetMathLibrary.BreakRotator` (`self.K2_GetActorRotation`)))
  (bind (_newrotation_x _newrotation_y) (`KismetMathLibrary.BreakVector2D` (`self.ClampCameraAngle` (`KismetMathLibrary.MakeVector2D` (+ ActionValue_X _returnvalue_yaw) (+ ActionValue_Y _returnvalue_pitch)) (`self.RotationMin`) (`self.RotationMax`))))
  (:`Triggered`
    (`self.K2_SetActorRotation` (`KismetMathLibrary.MakeRotator` 0.0 _newrotation_y _newrotation_x))))

(fn `UserConstructionScript`)

(fn `WriteRenderTexture`
  (params (Write :type Boolean))
  (bind _scenecapturecomponent2d (`self.SceneCaptureComponent2D`))
  (if Write
    (set `SceneCaptureComponent2D.TextureTarget` "/Game/Art/Materials/Camera/RT_Camera.RT_Camera" _scenecapturecomponent2d)
    (else
      (set `SceneCaptureComponent2D.TextureTarget` null _scenecapturecomponent2d))))
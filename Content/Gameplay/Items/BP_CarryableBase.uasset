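; Base physics prop that a BP_Character can pick up, one at a time, and that deals impact damage.
; Interact claims the prop, and multicasts snap it to the holder's HoldPoint or restore physics on detach.
; Weight class presets or custom stats set mass, throw and damage values.
; Fast hits damage the prop, destroying it if Destructible, and hurt characters on a cooldown; the smooth pull-to-hand code is disconnected.
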(event `self.ReceiveHit`
  (params (MyComp :type "PrimitiveComponent Object Reference") (Other :type "Actor Object Reference") (OtherComp :type "PrimitiveComponent Object Reference") (bSelfMoved :type Boolean) (HitLocation :type "Vector Structure") (HitNormal :type "Vector Structure") (NormalImpulse :type "Vector Structure") (Hit :type "HitResult Structure (by ref)"))
  ; Applique des degats quand touche quelque chose + rebond (un joueur en gros)
  (if (`self.DealsImpactDamage`)
    (if (`self.CanDealImpactNow`)
      (bind _returnvalue (`PrimitiveComponent.GetPhysicsLinearVelocity` (`self.PropMesh`) "None"))
      (if (>= (`KismetMathLibrary.VSize` _returnvalue) (`self.MinSpeedToDealAnyDamage`))
        (`self.ReceivePropDamage` (`self.SelfImpactDamage`))
        (bind _asbp_character (cast `/Game/Character/BP_Character` Other))
        (set `self.CanDealImpactNow` false)
        (`/Game/Character/BP_Character.Server_ReceiveDamage` _asbp_character (`self.ImpactDamage`))
        (`KismetSystemLibrary.PrintString` "\"Impact damage\" ")
        (`KismetSystemLibrary.K2_SetTimer` null "ResetImpactDamageCooldown" (`self.ImpactDamageCooldown`))))))

(event `self.ReceiveBeginPlay`
  ; Appliquer la vie et les stats du props
  (set `self.CurrentHealth` (`self.MaxHealth`))
  (`self.ApplyWeightSettings`))

(event `self.ReceiveTick`
  (params (DeltaSeconds :type "Float (single-precision)"))
  ; Effet The Finals (props qui bouge du sol jusqu'a la main)
)

(event `/Game/Gameplay/Interaction/BPI_Interactable.Interact`
  (params (Interactor :type "Actor Object Reference"))
  ; Interagir avec un prop
  (bind _asbp_character (cast `/Game/Character/BP_Character` Interactor))
  (bind _output_get (set `self.CharRef` _asbp_character))
  (`/Engine/EditorBlueprintResources/StandardMacros.IsValid` (`/Game/Character/BP_Character.HeldProp` _output_get)
    (:`Is Not Valid`
      (set `/Game/Character/BP_Character.HeldProp` self (`self.CharRef`))
      (set `self.LastHolder` (`self.CharRef`))
      (`self.SetReplicateMovement` false)
      (`self.ForceNetUpdate`)
      (`self.FlushNetDormancy`)
      (`self.Multicast_AttachToHolder` (`self.CharRef`)))))

(event `Multicast_AttachToHolder`
  (params (Carrier :type "/Game/Character/BP_Character Object Reference"))
  (bind _propmesh (`self.PropMesh`))
  (`PrimitiveComponent.SetSimulatePhysics` _propmesh false)
  (`PrimitiveComponent.SetCollisionEnabled` _propmesh "NoCollision")
  (`self.SetActorEnableCollision` false)
  (`self.K2_AttachToComponent` (`/Game/Character/BP_Character.HoldPoint` Carrier) "None" "SnapToTarget" "SnapToTarget" "KeepWorld" false)
  (set `self.MoveToHolder` false)
  (set `self.IsHeld` true))

(event `Multicast_DetachFromHolder`
  (`self.K2_DetachFromActor` "KeepWorld" "KeepWorld" "KeepWorld")
  (`self.SetActorEnableCollision` true)
  (`PrimitiveComponent.SetCollisionEnabled` (`self.PropMesh`) "QueryAndPhysics")
  (`PrimitiveComponent.SetSimulatePhysics` (`self.PropMesh`) true)
  (set `self.IsHeld` false)
  (set `self.MoveToHolder` false))

(fn `ApplyWeightSettings`
  ; Par default, utilisation des stats pré fait, si prop custom on coche UseCustomStats
  (if (not (`self.UseCustomStats`))
    (switch `/Game/Gameplay/Items/E_CarryableWeightClass` (`self.WeightClass`)
      (:`NewEnumerator0`
        (set `self.MassMultiplier` 0.5)
        (set `self.PickupMoveSpeed` 18.0)
        (set `self.ThrowForce` 2200.0)
        (set `self.MinSpeedToDealAnyDamage` 800.0)
        (set `self.SelfImpactDamage` 3.0)
        (set `self.ImpactDamage` 200.0))
      (:`NewEnumerator1`
        (set `self.MassMultiplier` 1.0)
        (set `self.PickupMoveSpeed` 15.0)
        (set `self.ThrowForce` 1500.0)
        (set `self.MinSpeedToDealAnyDamage` 500.0)
        (set `self.SelfImpactDamage` 2.0)
        (set `self.ImpactDamage` 10.0))
      (:`NewEnumerator2`
        (set `self.MassMultiplier` 2.0)
        (set `self.PickupMoveSpeed` 10.0)
        (set `self.ThrowForce` 900.0)
        (set `self.MinSpeedToDealAnyDamage` 300.0)
        (set `self.SelfImpactDamage` 2.0)
        (set `self.ImpactDamage` 200.0))))
  (`PrimitiveComponent.SetMassScale` (`self.PropMesh`) "None" (`self.MassMultiplier`)))

(fn `CanInteract`
  (params (Interactor :type "Actor Object Reference"))
  (returns (`Return Value` :type Boolean))
  ; Si Props déja en main impossible d'en prendre un autre, lacher celui en main avant
  (bind _asbp_character (cast `/Game/Character/BP_Character` Interactor)
    (:`then`
      (`/Engine/EditorBlueprintResources/StandardMacros.IsValid` (`/Game/Character/BP_Character.HeldProp` _asbp_character)
        (:`Is Valid`
          (return false))
        (:`Is Not Valid`
          (return true))))
    (:`CastFailed`
      (return false))))

(fn `ReceivePropDamage`
  (params (DamageAmount :type "Float (double-precision)"))
  ; Recoit des degats quand touche quelque chose, se casse si plus de vie pour objet fragile
  (bind _output_get (set `self.CurrentHealth` (- (`self.CurrentHealth`) (`self.DamageAmount`))))
  (`KismetSystemLibrary.PrintString` "\"Prop took damage: \" + DamageAmount + \" | HP left: \" + CurrentHealth")
  (if (<= _output_get 0.0)
    (if (`self.Destructible`)
      (`KismetSystemLibrary.PrintString` "\"Prop destroyed\"")
      (`self.K2_DestroyActor`))))

(fn `ResetImpactDamageCooldown`
  (set `self.CanDealImpactNow` true))

(fn `UserConstructionScript`)
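; Keycard-locked door that characters open by interacting, with access rules that depend on their team.
; A held keycard is required: Attackers spend one of its limited uses per opening, while Defenders open without consuming any.
; OpenDoor sets IsOpen and starts a timer to close it again; CanInteract refuses interaction while open.
; The IsOpen RepNotify calls UpdateDoorVisual, which snaps the hinge between open and closed yaw.
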(event `TryOpenFromInteractor`
  (params (Interactor :type "Actor Object Reference"))
  (bind _usesremaining_attackers (`/Game/Gameplay/Items/Keycard/BP_KeycardPickup.UsesRemaining_Attackers` (`/Game/Character/BP_Character.HeldKeycard` (`self.CharRef`))))
  ; Interaction avec la porte SEULEMENT si on a une keycard et en fonction du nombre d'utilisation (système avec bouton pour ouvrir la porte)
  (bind _asbp_character (cast `/Game/Character/BP_Character` Interactor))
  (bind _output_get (set `self.CharRef` _asbp_character))
  (if (`KismetSystemLibrary.IsValid` (`/Game/Character/BP_Character.HeldKeycard` _output_get))
    (switch `/Game/Gameplay/E_Player_Team` (`/Game/Character/BP_Character.Team` (`self.CharRef`))
      (:`NewEnumerator0`
        (if (> _usesremaining_attackers 0)
          (set `/Game/Gameplay/Items/Keycard/BP_KeycardPickup.UsesRemaining_Attackers` (- _usesremaining_attackers 1) (`/Game/Character/BP_Character.HeldKeycard` (`self.CharRef`)))
          (`KismetSystemLibrary.PrintString` (`KismetStringLibrary.Conv_IntToString` (`/Game/Gameplay/Items/Keycard/BP_KeycardPickup.UsesRemaining_Attackers` (`/Game/Character/BP_Character.HeldKeycard` (`self.CharRef`)))))
          (`self.OpenDoor`)
          (else
            (`KismetSystemLibrary.PrintString` "No uses left"))))
      (:`NewEnumerator1`
        (`self.OpenDoor`)))
    (else
      (`KismetSystemLibrary.PrintString` "Need keycard"))))

(event `/Game/Gameplay/Interaction/BPI_Interactable.Interact`
  (params (Interactor :type "Actor Object Reference"))
  ; Interaction avec la porte SEULEMENT si on a une keycard et en fonction du nombre d'utilisation
  (`self.TryOpenFromInteractor` Interactor))

(event `OpenDoor`
  ; Ouvrir/fermer la porte (avec un timer d'ouverture)
  (if (not (`self.IsOpen`))
    (set `self.IsOpen` true)
    (`KismetSystemLibrary.K2_SetTimer` null "CloseDoor" (`self.OpenDuration`))))

(event `CloseDoor`
  ; Ouvrir/fermer la porte (avec un timer d'ouverture)
  (set `self.IsOpen` false))

(fn `CanInteract`
  (params (Interactor :type "Actor Object Reference"))
  (returns (`Return Value` :type Boolean))
  (cast `/Game/Character/BP_Character` Interactor
    (:`then`
      (if (`self.IsOpen`)
        (return false)
        (else
          (return true))))
    (:`CastFailed`
      (return false))))

(fn `OnRep_IsOpen`
  (`self.UpdateDoorVisual`))

(fn `UpdateDoorVisual`
  (`KismetSystemLibrary.PrintString` "UPDATE DOOR VISUAL")
  (if (`self.IsOpen`)
    (`SceneComponent.K2_SetRelativeRotation` (`self.Hinge`) (`KismetMathLibrary.MakeRotator` 0.0 0.0 (`self.OpenYaw`)) false false)
    (else
      (`SceneComponent.K2_SetRelativeRotation` (`self.Hinge`) (`KismetMathLibrary.MakeRotator` 0.0 0.0 (`self.ClosedYaw`)) false false))))

(fn `UserConstructionScript`)
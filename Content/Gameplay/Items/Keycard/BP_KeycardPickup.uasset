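; BP_KeycardPickup is an interactable keycard item that a BP_Character picks up, limited to one held keycard at a time.
; CanInteract allows interaction only for a BP_Character without a valid HeldKeycard.
; Interact repeats that check and stores the keycard as the character's HeldKeycard.
; For the Attacker team only, it then hides the actor and disables its collision and cube physics, with no handling for other teams.
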(event `/Game/Gameplay/Interaction/BPI_Interactable.Interact`
  (params (Interactor :type "Actor Object Reference"))
  ; Interaction keycard (si déja une clé ou pas) + en fonction de la team pour utilisations
  (`KismetSystemLibrary.PrintString` "\"INTERACT OK\"")
  (bind _asbp_character (cast `/Game/Character/BP_Character` Interactor))
  (bind _output_get (set `self.CharRef` _asbp_character))
  (if (`KismetSystemLibrary.IsValid` (`/Game/Character/BP_Character.HeldKeycard` _output_get))
    (`KismetSystemLibrary.PrintString` "Already has a keycard")
    (else
      (set `/Game/Character/BP_Character.HeldKeycard` self _output_get)
      (switch `/Game/Gameplay/E_Player_Team` (`/Game/Character/BP_Character.Team` _output_get)
        (:`NewEnumerator0`
          (`self.SetActorHiddenInGame` true)
          (`self.SetActorEnableCollision` false)
          (`PrimitiveComponent.SetSimulatePhysics` (`self.Cube`) false))))))

(fn `CanInteract`
  (params (Interactor :type "Actor Object Reference"))
  (returns (`Return Value` :type Boolean))
  ; Si deja keycard sur soi = impossible // Si pas de keycard = autorisé a pickup
  (bind _asbp_character (cast `/Game/Character/BP_Character` Interactor)
    (:`then`
      (`/Engine/EditorBlueprintResources/StandardMacros.IsValid` (`/Game/Character/BP_Character.HeldKeycard` _asbp_character)
        (:`Is Valid`
          (return false))
        (:`Is Not Valid`
          (return true))))
    (:`CastFailed`
      (return false))))

(fn `UserConstructionScript`)
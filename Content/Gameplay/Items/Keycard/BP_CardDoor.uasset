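; BP_CardDoor is a hinged door that opens through ForceOpenDoor, or through Interact when direct interaction is enabled, then closes itself on a timer.
; OpenDoor and CloseDoor set IsOpen and call ApplyDoorState, which plays or reverses a timeline meant to smoothly swing the hinge yaw.
; OnRep_IsOpen calls the same ApplyDoorState for multiplayer.
; CanInteract accepts only BP_Character on a closed, direct-interact door; UpdateDoorVisual is an unused stub.
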(event `ForceOpenDoor`
  ; Utiliser pour ouvrir porte avec bouton
  (`self.OpenDoor`))

(event `/Game/Gameplay/Interaction/BPI_Interactable.Interact`
  (params (Interactor :type "Actor Object Reference"))
  ; Ouvrir une porte sans bouton/cle juste interagir avec
  (if (`self.DirectInteractEnabled`)
    (`self.ForceOpenDoor`)))

(event `ApplyDoorState`
  ; Jouer la timeline
  (if (`self.IsOpen`)
    (`TimelineComponent.PlayFromStart` (`self.TL_DoorOpen`))
    (else
      (`TimelineComponent.Reverse` (`self.TL_DoorOpen`)))))

(event `CloseDoor`
  ; Ouvrir/fermer la porte (avec un timer d'ouverture + timeline pour effet smooth)
  (set `self.IsOpen` false)
  (`self.ApplyDoorState`))

(event `OpenDoor`
  ; Ouvrir/fermer la porte (avec un timer d'ouverture + timeline pour effet smooth)
  (if (not (`self.IsOpen`))
    (set `self.IsOpen` true)
    (`self.ApplyDoorState`)
    (`KismetSystemLibrary.K2_SetTimer` null "CloseDoor" (`self.OpenDuration`))))

(fn `CanInteract`
  (params (Interactor :type "Actor Object Reference"))
  (returns (`Return Value` :type Boolean))
  (cast `/Game/Character/BP_Character` Interactor
    (:`then`
      (if (`self.DirectInteractEnabled`)
        (if (`self.IsOpen`)
          (return false)
          (else
            (return true)))
        (else
          (return false))))
    (:`CastFailed`
      (return false))))

(fn `OnRep_IsOpen`
  ; Timeline fonctionnelle multi-ready
  (`self.ApplyDoorState`))

(fn `UpdateDoorVisual`)

(fn `UserConstructionScript`)
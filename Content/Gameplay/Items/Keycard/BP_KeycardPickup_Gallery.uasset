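; BP_KeycardPickup_Gallery is an interactable keycard pickup that a character can carry, one at a time.
; On interact it stores itself as the character's HeldKeycard, shows an acquired popup through the controller, then hides and disables collision and physics for Thief and Employee alike.
; It supplies interaction checks, name text and sound, highlights its cube through custom depth stencil, and can reset its attacker use count.
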(event `/Game/Gameplay/Interaction/BPI_Interactable.Interact`
  (params (Interactor :type "Actor Object Reference"))
  ; Interaction keycard (si déja une clé ou pas) + en fonction de la team pour utilisations
  (bind _asbp_character (cast `/Game/Character/BP_Character` Interactor))
  (bind _output_get (set `self.CharRef` _asbp_character))
  (if (not (`KismetSystemLibrary.IsValid` (`/Game/Character/BP_Character.HeldKeycard` _output_get)))
    (set `/Game/Character/BP_Character.HeldKeycard` self _output_get)
    (bind _asbp_character_controller (cast `/Game/Character/Control/BP_CharacterController` (`Pawn.GetController` _output_get)))
    (`/Game/Character/Control/BP_CharacterController.Client_ShowActionPopup` _asbp_character_controller (`|FormatText` "{Key} acquired" (`self.KeycardName`)))
    (bind _team (`/Game/Character/BP_Character.GetCurrentTeam` _asbp_character))
    (switch `ETeam` _team
      (:`Thief`
        _)
      (:`Employee`
        _))
    (`self.SetActorHiddenInGame` true)
    (`self.SetActorEnableCollision` false)
    (`PrimitiveComponent.SetSimulatePhysics` (`self.Cube`) false)))

(event `/Game/Gameplay/Interaction/BPI_Interactable.SetOutlineEnable`
  (params (Enable :type Boolean))
  (bind _cube (`self.Cube`))
  ; Outline
  (`PrimitiveComponent.SetRenderCustomDepth` _cube Enable)
  (`PrimitiveComponent.SetCustomDepthStencilValue` _cube 1))

(fn `CanInteract`
  (params (Interactor :type "Actor Object Reference"))
  (returns (`Return Value` :type Boolean))
  ; Si deja keycard sur soi = impossible // Si pas de keycard = autorisé a pickup
  (bind _asbp_character (cast `/Game/Character/BP_Character` Interactor)
    (:`then`
      (`/Engine/EditorBlueprintResources/StandardMacros.IsValid` (`/Game/Character/BP_Character.HeldKeycard` _asbp_character)
        (:`Is Valid`
          (return false))
        (:`Is Not Valid`
          (return true))))
    (:`CastFailed`
      (return false))))

(fn `GetInteractionText`
  (params (Interactor :type "Actor Object Reference"))
  (returns (InteractionText :type Text))
  ; Text a afficher quand on vise la keycard
  (return (`|FormatText` "{Key}" (`self.KeycardName`))))

(fn `ResetKeycardUses`
  (set `self.UsesRemaining_Attackers` 3))

(fn `ShouldPlayInteractionSound`
  (returns (Bool :type Boolean))
  (return true))

(fn `UserConstructionScript`)
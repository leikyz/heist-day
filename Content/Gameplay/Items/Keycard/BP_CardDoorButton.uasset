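; Interactable keycard button that force-opens its linked doors when none are open and the character holds the required keycard type.
; Attackers spend one keycard use per press, refreshed on their HUD through the controller, while Defenders open doors without spending uses.
; A wrong or missing keycard triggers an error sound and client popup.
; It also supplies interaction checks, prompt text and a custom-depth outline.
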(event `/Game/Gameplay/Interaction/BPI_Interactable.Interact`
  (params (Interactor :type "Actor Object Reference"))
  ; Ouverture porte + consommation d'une seule utilisation par bouton de keycard + message popup
  (if (> (`KismetArrayLibrary.Array_Length` (`self.LinkedDoors`)) 0)
    (bind _return_value (`self.AreAnyLinkedDoorsOpen`))
    (if (not _return_value)
      (bind _asbp_character (cast `/Game/Character/BP_Character` Interactor))
      (bind _heldkeycard (`/Game/Character/BP_Character.HeldKeycard` _asbp_character))
      (`/Engine/EditorBlueprintResources/StandardMacros.IsValid` _heldkeycard
        (:`Is Valid`
          (if (`|EnumEquality` (`/Game/Gameplay/Items/Keycard/BP_KeycardPickup.KeycardType` _heldkeycard) (`self.RequiredKeycardType`))
            (switch `/Game/Gameplay/E_Player_Team` (`/Game/Character/BP_Character.Team` _asbp_character)
              (:`NewEnumerator0`
                (bind _usesremaining_attackers (`/Game/Gameplay/Items/Keycard/BP_KeycardPickup.UsesRemaining_Attackers` (`/Game/Character/BP_Character.HeldKeycard` _asbp_character)))
                (if (> _usesremaining_attackers 0)
                  (bind _output_get (set `/Game/Gameplay/Items/Keycard/BP_KeycardPickup.UsesRemaining_Attackers` (- _usesremaining_attackers 1) (`/Game/Character/BP_Character.HeldKeycard` _asbp_character)))
                  (bind _asbp_character_controller (cast `/Game/Character/Control/BP_CharacterController` (`Pawn.GetController` _asbp_character)))
                  (`/Game/Character/Control/BP_CharacterController.Client_RefreshKeycardUsesHUD` _asbp_character_controller _output_get)
                  (for _array_element (`self.LinkedDoors`)
                    (`/Engine/EditorBlueprintResources/StandardMacros.IsValid` _array_element
                      (:`Is Valid`
                        (`/Game/Gameplay/Items/Keycard/BP_CardDoor.ForceOpenDoor` _array_element))))))
              (:`NewEnumerator1`
                (for _array_element_2 (`self.LinkedDoors`)
                  (`/Engine/EditorBlueprintResources/StandardMacros.IsValid` _array_element_2
                    (:`Is Valid`
                      (`/Game/Gameplay/Items/Keycard/BP_CardDoor.ForceOpenDoor` _array_element_2))))))
            (else
              (bind _asbp_character_controller_2 (cast `/Game/Character/Control/BP_CharacterController` (`Pawn.GetController` _asbp_character)))
              (`self.MC_PlayInvalidUseSound`)
              (`/Game/Character/Control/BP_CharacterController.Client_ShowActionPopup` _asbp_character_controller_2 "Wrong Keycard"))))
        (:`Is Not Valid`
          (bind _asbp_character_controller_3 (cast `/Game/Character/Control/BP_CharacterController` (`Pawn.GetController` _asbp_character)))
          (`self.MC_PlayInvalidUseSound`)
          (`/Game/Character/Control/BP_CharacterController.Client_ShowActionPopup` _asbp_character_controller_3 "Need Keycard"))))))

(event `/Game/Gameplay/Interaction/BPI_Interactable.SetOutlineEnable`
  (params (Enable :type Boolean))
  ; Outline
  (`PrimitiveComponent.SetRenderCustomDepth` (`self.ButtonMesh`) Enable))

(event `MC_PlayValidUseSound`
  ; Son quand keycard validé
  (`GameplayStatics.PlaySoundAtLocation` (`self.ValidUseSound`) (`self.K2_GetActorLocation`) (struct) 1.0 1.0 0.0 null null null null))

(event `MC_PlayInvalidUseSound`
  ; Son quand pas la bonne keycard
  (`GameplayStatics.PlaySoundAtLocation` (`self.UnvalidUseSound`) (`self.K2_GetActorLocation`) (struct) 1.0 1.0 0.0 null null null null))

(fn `AreAnyLinkedDoorsOpen`
  (returns (`Return Value` :type Boolean))
  (set `self.AnyOpen` false)
  (for _array_element (`self.LinkedDoors`)
    (`/Engine/EditorBlueprintResources/StandardMacros.IsValid` _array_element
      (:`Is Valid`
        (if (`/Game/Gameplay/Items/Keycard/BP_CardDoor.IsOpen` _array_element)
          (bind _output_get (set `self.AnyOpen` true))
          (break)))))
  (return _output_get))

(fn `CanInteract`
  (params (Interactor :type "Actor Object Reference"))
  (returns (`Return Value` :type Boolean))
  (locals (NewLocalVar :type "Array of /Game/Gameplay/Items/Keycard/BP_CardDoor Object Reference"))
  (cast `/Game/Character/BP_Character` Interactor
    (:`then`
      (if (> (`KismetArrayLibrary.Array_Length` (`self.LinkedDoors`)) 0)
        (bind _return_value (`self.AreAnyLinkedDoorsOpen`))
        (if (== _return_value false)
          (return true)
          (else
            (return false)))))
    (:`CastFailed`
      (return false))))

(fn `GetInteractionText`
  (params (Interactor :type "Actor Object Reference"))
  (returns (InteractionText :type Text))
  ; Text a afficher quand on vise le bouton avec une keycard sur soi
  (bind _asbp_character (cast `/Game/Character/BP_Character` Interactor)
    (:`then`
      (`/Engine/EditorBlueprintResources/StandardMacros.IsValid` (`/Game/Character/BP_Character.HeldKeycard` _asbp_character)
        (:`Is Valid`
          (return (`|FormatText` "Use Keycard")))
        (:`Is Not Valid`
          (return (`|FormatText` "")))))
    (:`CastFailed`
      (return ""))))

(fn `ShouldPlayInteractionSound`
  (returns (Bool :type Boolean))
  (return false))

(fn `UserConstructionScript`)
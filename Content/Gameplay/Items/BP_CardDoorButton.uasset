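; BP_CardDoorButton is an interactable button that opens a linked door on behalf of the interacting character.
; CanInteract allows use only when the interactor is a BP_Character and a valid LinkedDoor is set.
; Interact forwards the interactor to the door's TryOpenFromInteractor, so the button itself holds no opening logic.
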(event `/Game/Gameplay/Interaction/BPI_Interactable.Interact`
  (params (Interactor :type "Actor Object Reference"))
  (`/Engine/EditorBlueprintResources/StandardMacros.IsValid` (`self.LinkedDoor`)
    (:`Is Valid`
      (`/Game/Gameplay/Items/BP_CardDoor.TryOpenFromInteractor` (`self.LinkedDoor`) Interactor))))

(fn `CanInteract`
  (params (Interactor :type "Actor Object Reference"))
  (returns (`Return Value` :type Boolean))
  (cast `/Game/Character/BP_Character` Interactor
    (:`then`
      (`/Engine/EditorBlueprintResources/StandardMacros.IsValid` (`self.LinkedDoor`)
        (:`Is Valid`
          (return true))
        (:`Is Not Valid`
          (return false))))
    (:`CastFailed`
      (return false))))

(fn `UserConstructionScript`)
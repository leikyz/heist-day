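; Prop actor that draws a throw trajectory line from a list of world-space path positions supplied by its caller.
; UpdateTrajectory destroys the previous segments, rebuilds TrajectorySpline from those positions, then spawns a thin spline mesh between each pair of points using SegmentMesh and SegmentMaterial.
; HideTrajectory destroys all segments and clears the spline; the actor computes no physics and does nothing on its own.
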(fn `HideTrajectory`
  (for _array_element (`self.SplineMeshes`)
    (`ActorComponent.K2_DestroyComponent` _array_element))
  (`KismetArrayLibrary.Array_Clear` (`self.SplineMeshes`))
  (`SplineComponent.ClearSplinePoints` (`self.TrajectorySpline`) true))

(fn `UpdateTrajectory`
  (params (PathPosition :type "Array of Vector Structure"))
  (bind _trajectoryspline (`self.TrajectorySpline`))
  (bind _trajectoryspline_2 (`self.TrajectorySpline`))
  (bind _splinemeshes (`self.SplineMeshes`))
  (for _array_element _splinemeshes
    (`ActorComponent.K2_DestroyComponent` _array_element))
  (`KismetArrayLibrary.Array_Clear` _splinemeshes)
  (`SplineComponent.ClearSplinePoints` (`self.TrajectorySpline`) true)
  (for _array_element_2 PathPosition
    (`SplineComponent.AddSplinePoint` (`self.TrajectorySpline`) _array_element_2 "World" false))
  (`SplineComponent.UpdateSpline` (`self.TrajectorySpline`))
  (for _index (range (+ (- (`SplineComponent.GetNumberOfSplinePoints` (`self.TrajectorySpline`)) 2) 1))
    (bind _returnvalue (`AddComponent|NODE_AddSplineMeshComponent-0` :`bManualAttachment` true))
    (`SceneComponent.SetMobility` _returnvalue "Movable")
    (`SceneComponent.K2_AttachToComponent` _returnvalue (`self.TrajectorySpline`) "None" "KeepRelative" "KeepRelative" "KeepRelative" true)
    (`StaticMeshComponent.SetStaticMesh` _returnvalue (`self.SegmentMesh`))
    (`PrimitiveComponent.SetMaterial` _returnvalue 0 (`self.SegmentMaterial`))
    (`SplineMeshComponent.SetStartScale` _returnvalue (0.03 0.03) true)
    (`SplineMeshComponent.SetEndScale` _returnvalue (0.03 0.03) true)
    (bind _returnvalue_2 (+ _index 1))
    (`SplineMeshComponent.SetStartAndEnd` _returnvalue (`SplineComponent.GetLocationAtSplinePoint` _trajectoryspline_2 _index "Local") (`SplineComponent.GetTangentAtSplinePoint` _trajectoryspline_2 _index "Local") (`SplineComponent.GetLocationAtSplinePoint` _trajectoryspline _returnvalue_2 "Local") (`SplineComponent.GetTangentAtSplinePoint` _trajectoryspline _returnvalue_2 "Local") true)
    (`KismetArrayLibrary.Array_Add` (`self.SplineMeshes`) _returnvalue)))

(fn `UserConstructionScript`)
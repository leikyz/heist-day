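; Base carryable prop that unarmed players can pick up, with a name, extraction value and outline highlight.
; Interacting records the holder and multicasts attachment to a hand socket; detaching restores physics and collision.
; On server hits, fast thrown props damage characters other than the last holder through the game mode, while other impacts wear down the prop, breaking destructible ones.
; Weight-class presets set mass, throw and impact stats unless custom stats are enabled.
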(event `self.ReceiveHit`
  (params (MyComp :type "PrimitiveComponent Object Reference") (Other :type "Actor Object Reference") (OtherComp :type "PrimitiveComponent Object Reference") (bSelfMoved :type Boolean) (HitLocation :type "Vector Structure") (HitNormal :type "Vector Structure") (NormalImpulse :type "Vector Structure") (Hit :type "HitResult Structure (by ref)"))
  ; Applique des degats quand touche quelque chose + rebond (un joueur en gros)
  (`/Engine/EditorBlueprintResources/ActorMacros.Switch Has Authority`
    (:`Authority`
      (if (`self.DealsImpactDamage`)
        (if (`self.CanDealImpactNow`)
          (bind _returnvalue (`PrimitiveComponent.GetPhysicsLinearVelocity` (`self.PropMesh`) "None"))
          (if (>= (`KismetMathLibrary.VSize` _returnvalue) (`self.MinSpeedToDealAnyDamage`))
            (bind _asbp_character (cast `/Game/Character/BP_Character` Other)
              (:`then`
                (if (!= _asbp_character (`self.LastHolder`))
                  (if (`self.IsThrown`)
                    (if (>= (`KismetMathLibrary.Vector_Distance` (`self.K2_GetActorLocation` _asbp_character) (`self.ThrowStartLocation`)) (`self.MinDistanceBeforeCanHitThrowerOrPlayers`))
                      (set `self.CanDealImpactNow` false)
                      (bind _asheist_day_game_mode (cast `HeistDayGameMode` (`GameplayStatics.GetGameMode`)))
                      ;; Update damage and replicates it to all clients (start respawn behaviour if needed)
                      (`HeistDayGameMode.HandlePlayerDamage` _asheist_day_game_mode (`Pawn.GetController` _asbp_character) (`Pawn.GetController` (`self.CharRef`)) 50.0)
                      (`/Game/Character/BP_Character.Server_PlayAnySound` _asbp_character "/Game/Audio/Sounds/Gameplay/ImpactSurJoueur.ImpactSurJoueur" (`self.K2_GetActorLocation` _asbp_character) 1.0 "/Game/Audio/AttenuationPresets/ATT_Foley.ATT_Foley" 1.0 0.0)
                      (if (`HeistDayPlayerState.IsDead` (`/Game/Character/BP_Character.As Heist Day Player State` _asbp_character))
                        (`/Game/Character/BP_Character.Server_HandleRespawn` _asbp_character))))))
              (:`CastFailed`
                (`self.ReceivePropDamage` (`self.SelfImpactDamage`))
                (if (`self.CanPlayHitSound`)
                  (set `self.CanPlayHitSound` false)
                  (`self.MC_PlayPropHitSound`)
                  (`KismetSystemLibrary.K2_SetTimer` null "ResetHitSoundCooldown" 0.5))))))))))

(event `RestorePawnCollision`
  ; Ignore Collision quand on lance le prop + au sol (que ca nous tue pas)
  (`PrimitiveComponent.SetCollisionResponseToChannel` (`self.PropMesh`) "ECC_Pawn" "ECR_Block"))

(event `self.PropMesh.OnComponentSleep`
  (params (SleepingComponent :type "PrimitiveComponent Object Reference") (BoneName :type Name))
  ; Ignore Collision quand on lance le prop + au sol (que ca nous tue pas)
  (set `self.IsThrown` false)
  (set `self.CanDealImpactNow` false))

(event `self.ReceiveBeginPlay`
  ; Appliquer la vie et les stats du props
  (set `self.CurrentHealth` (`self.MaxHealth`))
  (`self.ApplyWeightSettings`))

(event `MC_PlayPropHitSound`
  ; SON
  ;; Son quand prop hit quelque chose
  (`GameplayStatics.PlaySoundAtLocation` (`self.PropHitSound`) (`self.K2_GetActorLocation`) (struct) 0.3 1.0 0.0 null null null null))

(event `self.ReceiveTick`
  (params (DeltaSeconds :type "Float (single-precision)"))
  (bind _charref (`self.CharRef`))
  (bind _returnvalue (`SceneComponent.K2_GetComponentLocation` (`Character.Mesh` _charref)))
  (bind _returnvalue_2 (`KismetMathLibrary.VInterpTo` (`self.K2_GetActorLocation`) _returnvalue DeltaSeconds (`self.PickupMoveSpeed`)))
  ; Effet The Finals (props qui bouge du sol jusqu'a la main)
  (if (`self.MoveToHolder`)
    (`/Engine/EditorBlueprintResources/StandardMacros.IsValid` _charref
      (:`Is Valid`
        (`self.K2_SetActorLocation` _returnvalue_2)
        (if (<= (`KismetMathLibrary.Vector_Distance` _returnvalue_2 _returnvalue) (`self.AttachDistance`))
          (`self.K2_AttachToComponent` (`Character.Mesh` (`self.CharRef`)) "PropSocket_R" "SnapToTarget" "SnapToTarget" "KeepWorld" false)
          (set `self.MoveToHolder` false)
          (set `self.IsHeld` true))))))

(event `MC_PlayPropDestroySound`
  ; SON
  ;; Son quand le prop se détruit
  (`GameplayStatics.PlaySoundAtLocation` (`self.PropDestroySound`) (`self.K2_GetActorLocation`) (struct) 1.0 1.0 0.0 null null null null))

(event `/Game/Gameplay/Interaction/BPI_Interactable.Interact`
  (params (Interactor :type "Actor Object Reference"))
  ; Interagir avec un prop
  (bind _asbp_character (cast `/Game/Character/BP_Character` Interactor))
  (bind _output_get (set `self.CharRef` _asbp_character))
  (`/Engine/EditorBlueprintResources/StandardMacros.IsValid` (`/Game/Character/BP_Character.HeldProp` _output_get)
    (:`Is Not Valid`
      (set `/Game/Character/BP_Character.HeldProp` self (`self.CharRef`))
      (set `self.LastHolder` (`self.CharRef`))
      (`self.SetReplicateMovement` false)
      (`self.ForceNetUpdate`)
      (`self.FlushNetDormancy`)
      (`self.Multicast_AttachToHolder` (`self.CharRef`)))))

(event `Multicast_AttachToHolder`
  (params (Carrier :type "/Game/Character/BP_Character Object Reference"))
  (bind _propmesh (`self.PropMesh`))
  ; Attacher le prop au point donner
  (`PrimitiveComponent.SetSimulatePhysics` _propmesh false)
  (`PrimitiveComponent.SetCollisionEnabled` _propmesh "NoCollision")
  (`self.SetActorEnableCollision` false)
  (`self.K2_AttachToComponent` (`Character.Mesh` Carrier) "PropSocket_R" "SnapToTarget" "SnapToTarget" "KeepWorld" false)
  (set `self.MoveToHolder` false)
  (set `self.IsHeld` true))

(event `Multicast_DetachFromHolder`
  ; Detacher le prop du point quand drop/throw
  (`self.K2_DetachFromActor` "KeepWorld" "KeepWorld" "KeepWorld")
  (`self.SetActorEnableCollision` true)
  (`PrimitiveComponent.SetCollisionEnabled` (`self.PropMesh`) "QueryAndPhysics")
  (`PrimitiveComponent.SetSimulatePhysics` (`self.PropMesh`) true)
  (set `self.IsHeld` false)
  (set `self.MoveToHolder` false))

(event `/Game/Gameplay/Interaction/BPI_Interactable.SetOutlineEnable`
  (params (Enable :type Boolean))
  (bind _propmesh (`self.PropMesh`))
  ; Outline
  (`PrimitiveComponent.SetRenderCustomDepth` _propmesh Enable)
  (`PrimitiveComponent.SetCustomDepthStencilValue` _propmesh 1))

(fn `ApplyWeightSettings`
  ; Par default, utilisation des stats pré fait, si prop custom on coche UseCustomStats
  (if (not (`self.UseCustomStats`))
    (switch `/Game/Gameplay/Items/Props/E_CarryableWeightClass` (`self.WeightClass`)
      (:`NewEnumerator0`
        (set `self.MassMultiplier` 0.5)
        (set `self.PickupMoveSpeed` 18.0)
        (set `self.ThrowForce` 4000.0)
        (set `self.MinSpeedToDealAnyDamage` 500.0)
        (set `self.SelfImpactDamage` 3.0)
        (set `self.ImpactDamage` 30.0))
      (:`NewEnumerator1`
        (set `self.MassMultiplier` 1.0)
        (set `self.PickupMoveSpeed` 15.0)
        (set `self.ThrowForce` 3500.0)
        (set `self.MinSpeedToDealAnyDamage` 200.0)
        (set `self.SelfImpactDamage` 2.0)
        (set `self.ImpactDamage` 30.0))
      (:`NewEnumerator2`
        (set `self.MassMultiplier` 2.0)
        (set `self.PickupMoveSpeed` 10.0)
        (set `self.ThrowForce` 2500.0)
        (set `self.MinSpeedToDealAnyDamage` 200.0)
        (set `self.SelfImpactDamage` 2.0)
        (set `self.ImpactDamage` 30.0))))
  (`PrimitiveComponent.SetMassScale` (`self.PropMesh`) "None" (`self.MassMultiplier`)))

(fn `CanInteract`
  (params (Interactor :type "Actor Object Reference"))
  (returns (`Return Value` :type Boolean))
  ; Si Props déja en main ou une arme, impossible d'en prendre un autre, lacher celui en main avant
  (bind _asbp_character (cast `/Game/Character/BP_Character` Interactor)
    (:`then`
      (`/Engine/EditorBlueprintResources/StandardMacros.IsValid` (`/Game/Character/BP_Character.HeldProp` _asbp_character)
        (:`Is Valid`
          (return false))
        (:`Is Not Valid`
          (switch `/Game/Character/Animation/Enum/E_Weapon_Type` (`/Game/Character/BP_Character.E_WeaponType` _asbp_character)
            (:`NewEnumerator0`
              (return true))
            (:`NewEnumerator1`
              (return false))))))
    (:`CastFailed`
      (return false))))

(fn `EnableImpactDamage`
  (set `self.CanDealImpactNow` true))

(fn `GetInteractionText`
  (params (Interactor :type "Actor Object Reference"))
  (returns (InteractionText :type Text))
  ; Text a afficher quand on vise un prop
  (return (`|FormatText` "{NomDuProp} ({Value}$)" (`self.PropName`) (`self.ExtractionValue`))))

(fn `ReceivePropDamage`
  (params (DamageAmount :type "Float (double-precision)"))
  ; Recoit des degats quand touche quelque chose, se casse si plus de vie pour objet fragile
  (bind _output_get (set `self.CurrentHealth` (- (`self.CurrentHealth`) (`self.DamageAmount`))))
  (if (<= _output_get 0.0)
    (if (`self.Destructible`)
      (`self.MC_PlayPropDestroySound`)
      (`self.K2_DestroyActor`))))

(fn `ResetHitSoundCooldown`
  (set `self.CanPlayHitSound` true))

(fn `ResetImpactDamageCooldown`
  (set `self.CanDealImpactNow` true))

(fn `ShouldPlayInteractionSound`
  (returns (Bool :type Boolean))
  (return true))

(fn `UserConstructionScript`)
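; Base weapon actor that handles attaching, equipping and reloading, with firing, visuals, muzzle location and weapon type left as stubs or defaults.
; Equip and UnEquip toggle mesh visibility, set the character's weapon type and switch the owner's crosshair through a client call.
; Server reload sets a reloading flag and multicasts visuals, and FinishReload clears it.
; Multicast fire runs the visual hook and spawns a temporary impact decal.
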(event `Multicast_ReloadVisuals`
  (`self.Reload_Visuals`))

(event `Multicast_FireVisuals`
  (params (HitData :type "HitResult Structure"))
  (bind (_bblockinghit _binitialoverlap _time _distance _location _impactpoint _normal _impactnormal) (`GameplayStatics.BreakHitResult` HitData))
  (`self.Fire_Visuals`)
  (`GameplayStatics.SpawnDecalAtLocation` "/Game/NiagaraExamples/Gallery/Materials/M_QuixelDecal_Simple.M_QuixelDecal_Simple" (16.0 8.0 8.0) _impactpoint (`KismetMathLibrary.Conv_VectorToRotator` _impactnormal) 30.0))

(fn `AttachToCharacter`
  (params (Character :type "/Game/Character/BP_Character Object Reference"))
  (`self.K2_AttachToComponent` (`Character.Mesh` Character) "weapon_r" "SnapToTarget" "SnapToTarget" "KeepRelative")
  (`self.K2_SetActorRelativeRotation` (`self.WeaponRotationOffset`)))

(fn `Equip`
  (bind _bp_character (`self.BP_Character`))
  (`SceneComponent.SetHiddenInGame` (`self.SkeletalMesh`) false false)
  (`/Engine/EditorBlueprintResources/StandardMacros.IsValid` _bp_character
    (:`Is Valid`
      (`self.K2_AttachToComponent` (`Character.Mesh` _bp_character) "weapon_socket_r" "SnapToTarget" "SnapToTarget" "KeepRelative")
      (bind _weapontype (`self.GetWeaponType`))
      (set `/Game/Character/BP_Character.E_WeaponType` _weapontype _bp_character)
      (`self.ToggleCrosshair` true))))

(fn `FinishReload`
  (set `self.bIsReloading` false))

(fn `Fire_Server`
  (params (CameraLocation :type "Vector Structure") (CameraRotation :type "Rotator Structure") (MuzzleFlashLocation :type "Vector Structure")))

(fn `Fire_Visuals`)

(fn `GetMuzzleFlashLocation`
  (returns (MuzzleFlashLocation :type "Vector Structure"))
  (return (0.0 0.0 0.0)))

(fn `GetWeaponType`
  (returns (WeaponType :type "/Game/Character/Animation/Enum/E_Weapon_Type Enum"))
  (return "NewEnumerator0"))

(fn `Reload_Server`
  (set `self.bIsReloading` true)
  (`self.Multicast_ReloadVisuals`))

(fn `Reload_Visuals`)

(fn `ToggleCrosshair`
  (params (State :type Boolean))
  (bind _asbp_character (cast `/Game/Character/BP_Character` (`self.GetOwner`)))
  (`/Game/Character/BP_Character.Client_SetCrosshairVisible` _asbp_character State)
  (return))

(fn `UnEquip`
  (bind _bp_character (`self.BP_Character`))
  (`SceneComponent.SetHiddenInGame` (`self.SkeletalMesh`) true false)
  (`/Engine/EditorBlueprintResources/StandardMacros.IsValid` _bp_character
    (:`Is Valid`
      (set `/Game/Character/BP_Character.E_WeaponType` "NewEnumerator0" _bp_character)
      (`self.ToggleCrosshair` false))))

(fn `UserConstructionScript`)
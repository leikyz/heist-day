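; Rifle weapon Blueprint that reports its weapon type and implements firing and reloading.
; Fire and Reload play the weapon mesh animation plus a matching character montage, and are blocked by IsReloading, which Reload sets but this file never clears.
; Fire also restarts a tinted muzzle flash and line traces from the muzzle toward a distant point along the camera's view, debug-drawn with the hit result unused.
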(fn `Fire`
  (bind _returnvalue (`GameplayStatics.GetPlayerCameraManager` 0))
  (bind _muzzleflash (`self.MuzzleFlash`))
  (if (not (`self.bIsReloading`))
    (`SkeletalMeshComponent.PlayAnimation` (`self.SkeletalMesh`) "/Game/Weapons/Rifle/Animations/AM_Weap_Rifle_Fire.AM_Weap_Rifle_Fire" false)
    (`NiagaraComponent.SetVariableLinearColor` _muzzleflash "Flash Base Color" (make `LinearColor` 8.0 1.9 0.1 0.5))
    (`NiagaraComponent.ResetSystem` _muzzleflash)
    (`/Game/Character/BP_Character.PlayCharacterRifleFireMontage` (`self.BP_Character`))
    (`KismetSystemLibrary.LineTraceSingle` :`Start` (`SceneComponent.K2_GetComponentLocation` (`self.MuzzleFlash`)) :`End` (+ (`PlayerCameraManager.GetCameraLocation` _returnvalue) (* (`KismetMathLibrary.GetForwardVector` (`PlayerCameraManager.GetCameraRotation` _returnvalue)) (10000.0 10000.0 10000.0))) :`TraceChannel` "TraceTypeQuery1" :`DrawDebugType` "ForDuration")))

(fn `GetWeaponType`
  (returns (WeaponType :type "/Game/Character/Animation/Enum/E_Weapon_Type Enum"))
  (return "NewEnumerator1"))

(fn `Reload`
  (if (not (`self.bIsReloading`))
    (set `self.bIsReloading` true)
    (`SkeletalMeshComponent.PlayAnimation` (`self.SkeletalMesh`) "/Game/Weapons/Rifle/Animations/AM_Weap_Rifle_Reload.AM_Weap_Rifle_Reload" false)
    (`/Game/Character/BP_Character.PlayCharacterRifleReloadMontage` (`self.BP_Character`))))

(fn `UserConstructionScript`
  (`parent.UserConstructionScript`))
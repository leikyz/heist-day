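; A fracturable foliage pot, a child Blueprint that adds plant behavior to an inherited fracture impact.
; On TriggerFractureImpact it runs the parent logic, then detaches the Foliage component, enables physics simulation on it and knocks it away with a fixed velocity-change impulse.
; The impulse ignores the impact location, and the construction script only calls the parent.
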(event `self.TriggerFractureImpact`
  (params (ImpactLocation :type "Vector Structure"))
  (bind _foliage (`self.Foliage`))
  (`parent.TriggerFractureImpact` ImpactLocation)
  (`SceneComponent.K2_DetachFromComponent` (`self.Foliage`) "KeepRelative" "KeepRelative" "KeepRelative" true)
  (`PrimitiveComponent.SetSimulatePhysics` _foliage true)
  (`PrimitiveComponent.AddImpulse` _foliage (50.0 50.0 5.0) "None" true))

(fn `UserConstructionScript`
  (`parent.UserConstructionScript`))